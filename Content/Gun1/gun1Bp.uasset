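; Gun actor Blueprint for a laser gun with a set of child-actor rings that can be revealed individually.
; On BeginPlay or DeactRings it deactivates and hides the spinner and all ring child actors.
; The actRing2 and actRing3 events activate and show their ring, while actRing1 and AddRing1 are empty.
; Pressing Fire spawns a particle emitter attached to the gun mesh at a fixed offset.
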(event Custom|DeactRings
  (bind _spinner1bp (Variables|Default|Getspinner1Bp))
  (Components|Activation|Deactivate _spinner1bp)
  (Rendering|SetVisibility _spinner1bp false false))

(event Custom|AddRing1)

(event Custom|actRing3
  (bind _childactor3 (Variables|Default|GetChildActor3))
  (Components|Activation|Activate _childactor3 false)
  (Rendering|SetVisibility _childactor3 true false))

(event Custom|actRing1)

(event Custom|actRing2
  (bind _childactor2 (Variables|Default|GetChildActor2))
  (Components|Activation|Activate _childactor2 false)
  (Rendering|SetVisibility _childactor2 true false))

(event EventBeginPlay
  (bind _spinner1bp (Variables|Default|Getspinner1Bp))
  (Components|Activation|Deactivate _spinner1bp)
  (Rendering|SetVisibility _spinner1bp false false))

(event EventActorBeginOverlap
  (params (OtherActor :type Actor%20Object%20Reference)))

(event EventTick
  (params (DeltaSeconds :type Float%20%28single-precision%29)))

(event Input|ActionEvents|InputActionFire
  (params (Key :type Key%20Structure :default "AnyKey"))
  (:Pressed
    (Effects|SpawnEmitterAttached "/Game/FirstPersonBP/Particles/partTest1/partTest1.partTest1" (Variables|Default|GetlazerGun1_Export_1) "None" "-0.002348,-1403.724487,370.719940" "0,-89.999962, 0")))

(fn ConstructionScript)