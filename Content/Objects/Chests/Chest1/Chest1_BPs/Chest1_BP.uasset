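; Lootable chest actor with a hinged lid and parallel item and quantity arrays, with an event to remove items.
; The player entering the sphere gets an interact prompt and E input, but openLid is empty; the code that fills the BoxCont1 menu and plays the opening is disconnected.
; closeLid reverses a timeline rotating the Arrow component, flipping the axis by saved starting yaw, then removes the prompt.
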(event OnComponentBeginOverlap(Sphere)
  (params (OverlappedComponent :type Primitive%20Component%20Object%20Reference) (OtherActor :type Actor%20Object%20Reference) (OtherComp :type Primitive%20Component%20Object%20Reference) (OtherBodyIndex :type Integer) (bFromSweep :type Boolean) (SweepResult :type Hit%20Result%20Structure%20%28by%20ref%29))
  (bind _returnvalue (Game|GetPlayerController 0))
  ;[1 1 1] chestIputOverlap
  (if (== OtherActor (Game|GetPlayerCharacter 0))
    (bind _returnvalue_2 (UserInterface|CreateWidget "/Game/Objects/Chests/Chest1/Chest1_BPs/qInteract.qInteract_C" _returnvalue))
    (UserInterface|Viewport|AddtoViewport _returnvalue_2 0)
    (Input|EnableInput _returnvalue)))

(event OnComponentEndOverlap(Sphere)
  (params (OverlappedComponent :type Primitive%20Component%20Object%20Reference) (OtherActor :type Actor%20Object%20Reference) (OtherComp :type Primitive%20Component%20Object%20Reference) (OtherBodyIndex :type Integer))
  ;[1 1 1] chestIputOverlap
  (if (== (Game|GetPlayerCharacter 0) OtherActor)
    (Widget|RemovefromParent (stale OnComponentBeginOverlap(Sphere) _returnvalue_2))
    (Input|DisableInput (Game|GetPlayerController 0))))

(event Custom|openLid
  ;[1 1 1] openLid
)

(event Custom|removeItem
  (params (indexToRemove :type Integer))
  (Utilities|Array|RemoveIndex (Variables|Default|GetItemsInBox) indexToRemove)
  (Utilities|Array|RemoveIndex (Variables|Default|GetitemInBoxQuant) indexToRemove))

(event Custom|closeLid
  (bind _arrow (Variables|Default|GetArrow))
  (bind _arrow_2 (Variables|Default|GetArrow))
  (bind _returnvalue (Transformation|GetRelativeTransform _arrow))
  (bind (_location _rotation _scale) (Math|Transform|BreakTransform _returnvalue))
  (bind (_x _y _z) (Math|Vector|BreakVector _location))
  (bind _returnvalue_2 (Math|Vector|MakeVector 0.0 _y 0.0))
  (bind _returnvalue_3 (Math|Vector|MakeVector _x _y _z))
  ;[1 1 1] ChestLidOpen
  (Variables|Default|SetisOpen? false)
  (bind _newtrack_0 (Timeline|Timeline_0 ReverseFromEnd)
    (:Update
      (if (< (Variables|Default|GetstartZ) 0.0)
        (Transformation|SetRelativeTransform _arrow_2 (Math|Transform|MakeTransform _returnvalue_3 (Math|Vector|RotatorfromAxisandAngle _returnvalue_2 _newtrack_0) _scale) false false)
        (else
          (Transformation|SetRelativeTransform _arrow_2 (Math|Transform|MakeTransform _returnvalue_3 (Math|Vector|RotatorfromAxisandAngle (Math|Vector|NegateVector _returnvalue_2) _newtrack_0) _scale) false false))))
    (:Finished
      (Widget|RemovefromParent (stale OnComponentBeginOverlap(Sphere) _returnvalue_2)))))

(event EventBeginPlay)

(event EventActorBeginOverlap
  (params (OtherActor :type Actor%20Object%20Reference)))

(event EventTick
  (params (DeltaSeconds :type Float%20%28single-precision%29)))

(event Input|KeyboardEvents|H
  (params (Key :type Key%20Structure :default "AnyKey")))

(event Input|KeyboardEvents|E
  (params (Key :type Key%20Structure :default "AnyKey"))
  ;[1 1 1] OpenInput
  (:Pressed
    (CallFunction|OpenLid)))

(fn ConstructionScript)